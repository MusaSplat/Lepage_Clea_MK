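; BP_LapPointPlacer spawns BP_LapPoint actors along a spline, apparently to lay out lap points for a track.
; Its PlacePoint event first destroys and clears the previously placed points, so each call rebuilds the set.
; It then samples world-space spline transforms at normalized time steps derived from PointAmount, spawning a point at each and storing it in AllPoints.
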(event `PlacePoint`
  (bind _pointamount (`self.PointAmount`))
  (`|ExecutionSequence`
    (:`then_0`
      (for _array_element (`self.AllPoints`)
        (`self.K2_DestroyActor` _array_element))
      (`KismetArrayLibrary.Array_Clear` (`self.AllPoints`)))
    (:`then_1`
      (for _index (range (+ _pointamount 1))
        (bind _returnvalue (`|SpawnActorFromClass` "/Game/Blueprint/BP_LapPoint.BP_LapPoint_C" (`SplineComponent.GetTransformAtTime` (`self.Spline`) (/ _index _pointamount) "World" false false) "Undefined" "MultiplyWithRoot" null null))
        (`KismetArrayLibrary.Array_Add` (`self.AllPoints`) _returnvalue)))))

(fn `UserConstructionScript`)