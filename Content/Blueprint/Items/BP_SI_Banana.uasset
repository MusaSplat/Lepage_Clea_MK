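; BP_SI_Banana is a short-lived physics item that damages pawns it hits.
; On BeginPlay it enables physics on its Cube, applies a one-off AddForce along world Y as an acceleration change, and destroys itself after a short delay.
; When the Cube hits a Pawn, it calls Damage on the BP_AC_Damage_Manager component of that pawn's controller.
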(event `self.ReceiveBeginPlay`
  (`parent.ReceiveBeginPlay`)
  (`PrimitiveComponent.SetSimulatePhysics` (`self.Cube`) true)
  (`PrimitiveComponent.AddForce` (`self.Cube`) (0.0 500.0 0.0) "None" true)
  (`KismetSystemLibrary.Delay` 2.0)
  (`self.K2_DestroyActor`))

(event `self.Cube.OnComponentHit`
  (params (HitComponent :type "PrimitiveComponent Object Reference") (OtherActor :type "Actor Object Reference") (OtherComp :type "PrimitiveComponent Object Reference") (NormalImpulse :type "Vector Structure") (Hit :type "HitResult Structure (by ref)"))
  (bind _aspawn (cast `Pawn` OtherActor))
  (`/Game/Blueprint/BP_AC_Damage_Manager.Damage` (`self.GetComponentByClass` (`Pawn.GetController` _aspawn) "/Game/Blueprint/BP_AC_Damage_Manager.BP_AC_Damage_Manager_C")))

(fn `UserConstructionScript`
  (`parent.UserConstructionScript`))